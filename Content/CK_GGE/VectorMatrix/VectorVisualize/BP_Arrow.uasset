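; BP_Arrow is an actor that visualizes a Vector variable as an arrow drawn from the actor's location.
; The construction script puts the head at root plus Vector in world space, aims head and shaft along it, and scales shaft X by its length.
; Setting MoveVector acts as a one-shot toggle that shifts the root by Vector, then resets itself.
; The event graph contains only empty events.
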(event `self.ReceiveTick`
  (params (DeltaSeconds :type "Float (single-precision)")))

(fn `UserConstructionScript`
  (bind _defaultsceneroot (`self.DefaultSceneRoot`))
  (bind _returnvalue (`KismetMathLibrary.FindLookAtRotation` (`self.ZeroVector`) (`self.Vector`)))
  (`SceneComponent.K2_SetWorldLocation` (`self.Arrow_Head_DirX`) (+ (`SceneComponent.K2_GetComponentLocation` (`self.DefaultSceneRoot`)) (`self.Vector`)) false false)
  (`SceneComponent.K2_SetWorldRotation` (`self.Arrow_Head_DirX`) _returnvalue false false)
  (`SceneComponent.K2_SetWorldRotation` (`self.Arrow_Shaft_DirX`) _returnvalue false false)
  (`SceneComponent.SetRelativeScale3D` (`self.Arrow_Shaft_DirX`) (`KismetMathLibrary.MakeVector` (* (`KismetMathLibrary.VSize` (`self.Vector`)) 0.01) 1.0 1.0))
  (if (`self.MoveVector`)
    (`SceneComponent.K2_SetWorldLocation` _defaultsceneroot (+ (`SceneComponent.K2_GetComponentLocation` _defaultsceneroot) (`self.Vector`)) false false)
    (set `self.MoveVector` false)))