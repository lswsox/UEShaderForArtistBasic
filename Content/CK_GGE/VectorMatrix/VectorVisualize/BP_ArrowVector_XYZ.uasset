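; Visualizes three basis vectors with red, green and blue arrow heads that drive materials on a JadeToad and its cage.
; SetBasisVectors converts each head's world location into 2x2mCage local space and scales it by VectorScale into BasisX, BasisY and BasisZ.
; SetMaterials pushes these as vector material parameters to both JadeToad components.
; Construction Script and EditorTick rerun both steps, updating in-editor; runtime Tick does nothing.
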(event `/Game/CK_GGE/EditorTick/BPI_EditorTick.EditorTick`
  (`self.SetBasisVectors`)
  (`self.SetMaterials`))

(event `self.ReceiveTick`
  (params (DeltaSeconds :type "Float (single-precision)")))

(fn `SetBasisVectors`
  (bind _vectorscale (`self.VectorScale`))
  (bind _returnvalue (`SceneComponent.K2_GetComponentToWorld` (`self.2x2mCage`)))
  (set `self.BasisX` (* (`KismetMathLibrary.InverseTransformLocation` _returnvalue (`SceneComponent.K2_GetComponentLocation` (`self.R_Head`))) _vectorscale))
  (set `self.BasisY` (* (`KismetMathLibrary.InverseTransformLocation` _returnvalue (`SceneComponent.K2_GetComponentLocation` (`self.G_Head`))) _vectorscale))
  (set `self.BasisZ` (* (`KismetMathLibrary.InverseTransformLocation` _returnvalue (`SceneComponent.K2_GetComponentLocation` (`self.B_Head`))) _vectorscale)))

(fn `SetMaterials`
  (bind _jadetoad2x2mcage (`self.JadeToad2x2mCage`))
  (bind _jadetoad (`self.JadeToad`))
  (`MeshComponent.SetVectorParameterValueOnMaterials` _jadetoad2x2mcage "BasisX" (`self.BasisX`))
  (`MeshComponent.SetVectorParameterValueOnMaterials` _jadetoad2x2mcage "BasisY" (`self.BasisY`))
  (`MeshComponent.SetVectorParameterValueOnMaterials` _jadetoad2x2mcage "BasisZ" (`self.BasisZ`))
  (`MeshComponent.SetVectorParameterValueOnMaterials` _jadetoad "BasisX" (`self.BasisX`))
  (`MeshComponent.SetVectorParameterValueOnMaterials` _jadetoad "BasisY" (`self.BasisY`))
  (`MeshComponent.SetVectorParameterValueOnMaterials` _jadetoad "BasisZ" (`self.BasisZ`)))

(fn `UserConstructionScript`
  (`AddComponent|NODE_AddChildActorComponent-1`)
  (`self.SetBasisVectors`)
  (`self.SetMaterials`))